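; Player hero character that moves relative to control rotation, snaps to four facings by key, and attacks by punching or shooting.
; Overlapping a GunItem destroys it, spawns a gun on the GunSocket and switches to the gun animation class.
; The attack input then drives the gun instead of the punch flag.
; Left click moves MouseClickPoint to the cursor hit, but its spawn and cursor setup are disconnected.
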(event `InputAction|TriggerAttack`
  (params (Key :type "Key Structure" :default "AnyKey"))
  (bind _gun (`self.Gun`))
  (:`Pressed`
    (if (`self.HavingGun`)
      (`/Game/Gun/GunBP.StartFire` _gun)
      (else
        (set `self.IsPunching` true))))
  (:`Released`
    (if (`self.HavingGun`)
      (`/Game/Gun/GunBP.StopFire` _gun)
      (else
        (set `self.IsPunching` false)))))

(event `InputAxis|MoveForward`
  (params (AxisValue :type "Float (single-precision)"))
  (`self.AddMovementInput` (`KismetMathLibrary.GetForwardVector` (`self.GetControlRotation`)) AxisValue))

(event `InputAxis|MoveRight`
  (params (AxisValue :type "Float (single-precision)"))
  (`self.AddMovementInput` (`KismetMathLibrary.GetRightVector` (`self.GetControlRotation`)) AxisValue))

(event `InputAction|Left`
  (params (Key :type "Key Structure" :default "AnyKey"))
  (:`Pressed`
    (`self.K2_SetActorRotation` (struct :`Yaw` -90.0))))

(event `InputAction|Right`
  (params (Key :type "Key Structure" :default "AnyKey"))
  (:`Pressed`
    (`self.K2_SetActorRotation` (struct :`Yaw` 90.0))))

(event `InputAxis|TurnRight`
  (params (AxisValue :type "Float (single-precision)")))

(event `InputAction|Forward`
  (params (Key :type "Key Structure" :default "AnyKey"))
  (:`Pressed`
    (`self.K2_SetActorRotation` (struct))))

(event `InputAction|Back`
  (params (Key :type "Key Structure" :default "AnyKey"))
  (:`Pressed`
    (`self.K2_SetActorRotation` (struct :`Yaw` 180.0))))

(event `self.ReceiveBeginPlay`)

(event `self.ReceiveActorBeginOverlap`
  (params (OtherActor :type "Actor Object Reference"))
  (bind _asgun_item (cast `/Game/UI/GunItem` OtherActor))
  (set `self.HavingGun` true)
  (`self.K2_DestroyActor` _asgun_item)
  (bind _returnvalue (`|SpawnActorFromClass` "/Game/Gun/GunBP.GunBP_C" (`SceneComponent.K2_GetComponentToWorld` (`self.Mesh`)) "Undefined" "OverrideRootScale"))
  (bind _output_get (set `self.Gun` _returnvalue))
  (`self.K2_AttachToComponent` _output_get (`self.Mesh`) "GunSocket" "SnapToTarget" "SnapToTarget" "KeepWorld" true)
  (`SkeletalMeshComponent.SetAnimInstanceClass` (`self.Mesh`) "/Game/Hero/GunHeroAni.GunHeroAni_C"))

(event `InputAction|LeftMouseClicked`
  (params (Key :type "Key Structure" :default "AnyKey"))
  (:`Pressed`
    (`self.K2_SetActorLocation` (`self.MouseClickPoint`) (`.Location` (`GameplayStatics.BreakHitResult` (`PlayerController.GetHitResultUnderCursorByChannel` (`GameplayStatics.GetPlayerController` 0) "TraceTypeQuery1" true))) false false)))

(fn `UserConstructionScript`
  (bind _mesh (`self.Mesh`))
  (`SceneComponent.K2_AttachToComponent` (`self.LeftHand`) _mesh "hand_l" "SnapToTarget" "SnapToTarget" "KeepWorld" true)
  (`SceneComponent.K2_AttachToComponent` (`self.RightHand`) _mesh "hand_r" "SnapToTarget" "SnapToTarget" "KeepWorld" true))